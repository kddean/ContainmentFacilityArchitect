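; Wall_baseBP is a base actor for grid-snapped wall placement with valid and invalid preview materials.
; Its construction script rounds location to WorldGridSize, stores X/Y GridCoords, and compares them against every other wall.
; Each comparison overwrites CurrentMat, so the last wall checked decides the preview, while IntersectingObject keeps any match.
; Solidify switches to BaseMat and flags the wall solid; both paths call UpdateShaders, which is empty here.
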(event `self.ReceiveTick`
  (params (DeltaSeconds :type "Float (single-precision)")))

(event `Solidify`
  (set `self.IsSolidified` true)
  (set `self.CurrentMat` (`self.BaseMat`))
  (`self.UpdateShaders`))

(event `UpdateShaders`)

(fn `GetCoords`
  (returns (GridCoords :type "Vector2D Structure"))
  (return (`self.GridCoords`)))

(fn `UserConstructionScript`
  (`self.Snap to Grid`)
  (bind _outactors (`GameplayStatics.GetAllActorsOfClass` "wall_baseBP_C"))
  (for _array_element _outactors
    (if (!= _array_element self)
      (bind _gridcoords (`self.GetCoords` _array_element))
      (bind _output_get (set `self.IsIntersecting` (== _gridcoords (`self.GridCoords`) :`ErrorTolerance` 0.5)))
      (if _output_get
        (set `self.CurrentMat` "/Game/WallTestRelated/WallPreviewInvalid_mat.WallPreviewInvalid_mat")
        (set `self.IntersectingObject` _array_element)
        (else
          (set `self.CurrentMat` "/Game/WallTestRelated/WallPreviewValid_mat.WallPreviewValid_mat")))))
  (`self.UpdateShaders`))